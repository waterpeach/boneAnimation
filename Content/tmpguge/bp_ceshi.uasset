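; Test actor that animates a skeletal mesh to pick and place boxes in a 5x5 grid on a pallet (Bp_tuoPan).
; A looping timer spawns each Bp_target on the "hard" socket and passes its grid position to the ceshiani AnimInstance.
; A timeline drives AniAlpha, releasing the box when alpha starts falling, while Tick zeroes its rotation.
; Once the grid fills, the timer plays the first level sequence found.
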(event OnComponentBeginOverlap(ceshi)
  (params (OverlappedComponent :type Primitive%20Component%20Object%20Reference) (OtherActor :type Actor%20Object%20Reference) (OtherComp :type Primitive%20Component%20Object%20Reference) (OtherBodyIndex :type Integer) (bFromSweep :type Boolean) (SweepResult :type Hit%20Result%20Structure%20%28by%20ref%29)))

(event OnComponentEndOverlap(ceshi)
  (params (OverlappedComponent :type Primitive%20Component%20Object%20Reference) (OtherActor :type Actor%20Object%20Reference) (OtherComp :type Primitive%20Component%20Object%20Reference) (OtherBodyIndex :type Integer)))

(event Custom|play
  (params (tmpTarget :type Vector))
  (Variables|Default|SettmpStop false)
  (Variables|Default|SettmpAlpha 0.0)
  (bind _asceshiani (Utilities|Casting|CastToceshiani (Components|SkeletalMesh|GetAnimInstance (Variables|Default|Getceshi))))
  (Default|GetLocalPtsandAngle _asceshiani tmpTarget)
  (Default|SetTarget _asceshiani tmpTarget)
  (bind _新建轨道_0 (Timeline|时间轴 PlayFromStart)
    (:Update
      (Utilities|FlowControl|Sequence
        (:then_0
          (Variables|/Game/tmpguge/ceshiani.ceshiani_C|SetAniAlpha _asceshiani _新建轨道_0))
        (:then_1
          (if (< _新建轨道_0 (Variables|Default|GettmpAlpha))
            (CallFunction|解除拾取)))
        (:then_2
          (Variables|Default|SettmpAlpha _新建轨道_0))))))

(event Custom|xunhuan
  (CallFunction|CreateBox)
  (Utilities|Time|SetTimerbyEvent (delegate Custom|createBox) 5.1 true))

(event Custom|解除拾取
  (Transformation|DetachFromComponent (Variables|/Game/tmpguge/bp_target.bp_target_C|GetDefaultSceneRoot (Variables|Default|GetNewVar_0)) "KeepWorld" "KeepWorld" "KeepWorld" true)
  (Transformation|SetWorldLocation (Variables|/Game/tmpguge/bp_target.bp_target_C|GetDefaultSceneRoot (Variables|Default|GetNewVar_0)) (Variables|Default|GetcurentTarget) false false)
  (bind _outactors (Actor|GetAllActorsOfClass "/Game/tmpguge/bp_tuoPan.bp_tuoPan_C"))
  (Transformation|AttachComponentToComponent (Variables|Default|GetNewVar_0) (Variables|/Game/tmpguge/bp_tuoPan.bp_tuoPan_C|GetDefaultSceneRoot (Utilities|Array|Get(acopy) _outactors)) "None" "KeepWorld" "KeepWorld" "KeepWorld" true))

(event Custom|createBox
  (bind _inittarget (Variables|Default|GetInitTarget))
  (if (and (< (Variables|Default|Getcol) 5) (< (Variables|Default|Getrow) 5))
    (bind _returnvalue (Game|SpawnActorfromClass "/Game/tmpguge/bp_target.bp_target_C" (Math|Transform|MakeTransform (Variables|Default|Get初始位置)) "Undefined" "MultiplyWithRoot" 0 0))
    (bind _output_get (Variables|Default|SetNewVar_0 _returnvalue))
    (Transformation|AttachComponentToComponent _output_get (Variables|Default|Getceshi) "hard" "KeepWorld" "KeepWorld" "KeepWorld" true)
    (Utilities|FlowControl|Sequence
      (:then_0
        (bind _output_get_2 (Variables|Default|SetcurentTarget (Math|Vector|MakeVector (+ (.x _inittarget) (* (Variables|Default|Getrow) 100)) (+ (.y _inittarget) (* (Variables|Default|Getcol) 100)) (.z _inittarget))))
        (CallFunction|Play (+ _output_get_2 "85.000000,0.000000,90.000000")))
      (:then_1
        (Variables|Default|Setrow (+ (Variables|Default|Getrow) 1)))
      (:then_2
        (if (> (Variables|Default|Getrow) 4)
          (Variables|Default|Setcol (+ (Variables|Default|Getcol) 1))
          (Variables|Default|Setrow 0))))
    (else
      (CallFunction|播放车车))))

(event Custom|播放车车
  (bind _outactors (Actor|GetAllActorsOfClass "/Script/LevelSequence.LevelSequenceActor"))
  (Sequencer|Player|Play (Variables|/Script/LevelSequence.LevelSequenceActor|GetSequencePlayer (Utilities|Array|Get(acopy) _outactors)) :!class /Script/MovieScene.MovieSceneSequencePlayer))

(event EventBeginPlay
  (CallFunction|Xunhuan))

(event Collision|EventActorBeginOverlap
  (params (OtherActor :type Actor%20Object%20Reference)))

(event EventTick
  (params (DeltaSeconds :type Float%20%28single-precision%29))
  (Transformation|SetWorldRotation (Variables|/Game/tmpguge/bp_target.bp_target_C|GetDefaultSceneRoot (Variables|Default|GetNewVar_0)) "0, 0, 0" false false))

(fn ConstructionScript)